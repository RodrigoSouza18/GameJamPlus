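; Enemy spawner actor that spawns waves of EnemyIA enemies at its own transform.
; On BeginPlay it binds its SpawnEnemy event to the RespawnEnemy dispatcher on BP_TopDownGameMode, so the game mode triggers each wave.
; Each wave spawns a batch sized from EnemySpawned, then raises EnemyIncrement and adds it to EnemySpawned, so successive waves grow by an increasing amount.
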(event Custom|SpawnEnemy
  (for _index (range 0 (- (Variables|Default|GetEnemySpawned) 2))
    (Game|SpawnActorfromClass "/Game/EnemyAI/EnemyIA.EnemyIA_C" (Transformation|GetActorTransform) "Undefined" "MultiplyWithRoot" 0 0))
  (Math|Integer|IncrementInt (Variables|Default|GetEnemyIncrement)
    (:%20%20
      (Variables|Default|SetEnemySpawned (+ (Variables|Default|GetEnemySpawned) (Variables|Default|GetEnemyIncrement))))))

(event EventBeginPlay
  (bind _asbp_top_down_game_mode (Utilities|Casting|CastToBP_TopDownGameMode (Game|GetGameMode)))
  (EventDispatchers|BindEventtoRespawnEnemy _asbp_top_down_game_mode (delegate Custom|SpawnEnemy)))

(fn ConstructionScript)